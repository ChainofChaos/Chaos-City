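; BP_GameModeBase is a game mode Blueprint that puts the game's UI widgets on screen at load, game start and game over.
; Each of its three events creates a widget, passes it data and adds it to the viewport.
; The HUD receives Health as its health points, the start screen gets the start delay, and the end screen gets whether the player won.
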(event EventUILoad
  (bind _returnvalue (UserInterface|CreateWidget "/Game/Blueprints/Widgets/WBP_UI.WBP_UI_C"))
  (Variables|/Game/Blueprints/Widgets/WBP_UI.WBP_UI_C|SetHealthPoint _returnvalue (Variables|Default|GetHealth))
  (UserInterface|Viewport|AddtoViewport _returnvalue 0))

(event EventGameStart
  (bind _returnvalue (UserInterface|CreateWidget "/Game/Blueprints/Widgets/WBP_GameStart.WBP_GameStart_C"))
  (Default|SetStartDelay _returnvalue (Variables|Default|GetStartDelay))
  (UserInterface|Viewport|AddtoViewport _returnvalue 0))

(event EventGameOver
  (params (bPlayerWon :type Boolean))
  (bind _returnvalue (UserInterface|CreateWidget "/Game/Blueprints/Widgets/WBP_GameEnd.WBP_GameEnd_C"))
  (Default|SetPlayerWon _returnvalue bPlayerWon)
  (UserInterface|Viewport|AddtoViewport _returnvalue 0))

(fn ConstructionScript)